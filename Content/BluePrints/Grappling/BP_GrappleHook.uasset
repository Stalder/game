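; BP_GrappleHook is a grappling hook actor that flies in a straight line to a target actor and stops there.
; BeginPlay caches start and end points and sets the ProjectileMovement velocity toward the target at Speed.
; Tick compares squared travel distance with the target's current distance from the start, then snaps to the cached endpoint and zeroes velocity.
; DistanceToTarget returns the remaining distance to that endpoint.
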(event EventBeginPlay
  (Variables|Default|SetStartingLocation (Transformation|GetActorLocation))
  (Variables|Default|SetEndingLocation (Transformation|GetActorLocation (Variables|Default|GetTarget)))
  (Variables|Default|SetDirection (Math|Vector|Normalize (- (Variables|Default|GetEndingLocation) (Variables|Default|GetStartingLocation))))
  (Variables|/Script/Engine.MovementComponent|SetVelocity (Variables|Default|GetProjectileMovement) (* (Variables|Default|GetDirection) (Variables|Default|GetSpeed))))

(event EventTick
  (params (DeltaSeconds :type Float%20%28single-precision%29))
  (if (>= (Class|KismetMathLibrary|VectorDistanceSquared (Transformation|GetActorLocation) (Variables|Default|GetStartingLocation)) (Class|KismetMathLibrary|VectorDistanceSquared (Transformation|GetActorLocation (Variables|Default|GetTarget)) (Variables|Default|GetStartingLocation)))
    (Transformation|SetActorLocation (+ (Variables|Default|GetStartingLocation) (* (Variables|Default|GetDirection) (Math|Vector|Distance(Vector) (Variables|Default|GetStartingLocation) (Variables|Default|GetEndingLocation)))) false false)
    (Variables|/Script/Engine.MovementComponent|SetVelocity (Variables|Default|GetProjectileMovement) "0, 0, 0")))

(fn ConstructionScript)

(fn DistancetoTarget
  (return (Math|Vector|Distance(Vector) (Variables|Default|GetEndingLocation) (Transformation|GetActorLocation))))