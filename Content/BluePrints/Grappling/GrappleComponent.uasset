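; Grappling hook component for ThirdPersonCharacter that pulls the player toward grapple target actors.
; A four-state machine on Tick: while retracted it highlights the visible in-range target closest to the camera's forward direction, found by sphere overlap and line traces.
; AttemptGrapple spawns a hook and a cable line attached to the right hand.
; As the hook nears, the character hops, flies to the target from the apex, then is launched off on arrival.
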(event EventBeginPlay
  (bind _asthird_person_character (Utilities|Casting|CastToThirdPersonCharacter (Components|GetOwner)))
  (Variables|Default|SetOwningCharacter _asthird_person_character))

(event EventTick
  (params (DeltaSeconds :type Float%20%28single-precision%29))
  (switch Utilities|FlowControl|Switch|SwitchonEGrappleState (Variables|Default|GetGrappleState)
    (:NewEnumerator0
      (CallFunction|TickRetracted))
    (:NewEnumerator1
      (CallFunction|TickFiring))
    (:NewEnumerator2
      (CallFunction|TickNearingTarget))
    (:NewEnumerator3
      (CallFunction|TickonTarget))))

(fn TickRetracted
  (bind _outactors (Collision|SphereOverlapActors (Transformation|GetActorLocation (Variables|Default|GetOwningCharacter)) (Variables|Default|GetMaxGrappleDistance) (Utilities|Array|MakeArray "ObjectTypeQuery1") "/Game/BluePrints/Grappling/BP_GrappleTarget.BP_GrappleTarget_C"))
  (bind _target (CallFunction|FindBestTarget _outactors))
  ;[1 1 1] OPTIMIZE
  (bind _asbp_grapple_target (Utilities|Casting|CastToBP_GrappleTarget _target))
  (CallFunction|SetCurrentTarget _asbp_grapple_target))

(fn TickFiring
  (if (< (Default|DistancetoTarget (Variables|Default|GetGrappleHook)) (Variables|Default|GetStartJumpDistance))
    (Character|LaunchCharacter (Variables|Default|GetOwningCharacter) "0, 0,500.000000" false false)
    (Variables|Default|SetGrappleState "NewEnumerator2")))

(fn TickNearingTarget
  (if (<= (.z (Transformation|GetVelocity (Variables|Default|GetOwningCharacter))) 0.0)
    (Variables|Default|SetInitialDirection (Utilities|OwnertoTarget))
    (Variables|Default|SetGrappleState "NewEnumerator3")))

(fn TickonTarget
  (bind _initialdirection (Variables|Default|GetInitialDirection))
  (bind _returnvalue (* _initialdirection 1e+02))
  (if (< (Transformation|GetDistanceTo (Variables|Default|GetOwningCharacter) (Variables|Default|GetCurrentTarget)) (Variables|Default|GetEndJumpDistance))
    (Development|PrintString "< 100")
    (Character|LaunchCharacter (Variables|Default|GetOwningCharacter) (Math|Vector|MakeVector (.x _returnvalue) (.y _returnvalue) (Math|Float|Max(Float) (.z _returnvalue) 5e+02)) false true)
    (CallFunction|SetCurrentTarget)
    (Actor|DestroyActor (Variables|Default|GetGrappleLine))
    (Variables|Default|SetGrappleLine 0)
    (Actor|DestroyActor (Variables|Default|GetGrappleHook))
    (Variables|Default|SetGrappleHook 0)
    (Variables|Default|SetGrappleState "NewEnumerator0")
    (else
      (Variables|/Script/Engine.MovementComponent|SetVelocity (Pawn|GetMovementComponent (Variables|Default|GetOwningCharacter)) (* (Utilities|OwnertoTarget) (Variables|Default|GetCharacterGrappleSpeed))))))

(fn FindBestTarget
  (params (Targets :type Array%20of%20Actor%20Object%20References))
  (bind _owningcharacter (Variables|Default|GetOwningCharacter))
  (for _array_element Targets
    (LocalVariables|SetCurrentTarget%20%28Local%29 _array_element)
    (bind (_outhit _returnvalue) (Collision|LineTraceByChannel (Transformation|GetActorLocation (Variables|Default|GetOwningCharacter)) (Transformation|GetActorLocation (LocalVariables|GetCurrentTarget%20%28Local%29)) "TraceTypeQuery1" false (Utilities|Array|MakeArray (Variables|Default|GetOwningCharacter)) "None"))
    (if _returnvalue
      (if (== (.HitActor (Collision|BreakHitResult _outhit)) (LocalVariables|GetCurrentTarget%20%28Local%29))
        (Utilities|FlowControl|Sequence
          (:then_0
            ;[1 1 1] Step 1) Calculate Angle to a target
            (LocalVariables|SetCurrentAngle%20%28Local%29 (Class|KismetMathLibrary|DegAcos (Math|Vector|DotProduct (Math|Vector|Normalize (- (Transformation|GetActorLocation (LocalVariables|GetCurrentTarget%20%28Local%29)) (Transformation|GetActorLocation _owningcharacter))) (Math|Vector|GetForwardVector (Variables|/Game/ThirdPersonBP/Blueprints/ThirdPersonCharacter.ThirdPersonCharacter_C|GetFollowCamera _owningcharacter))))))
          (:then_1
            ;[1 1 1] Step 2) Check if current angle is min & buffer min angle
            (if (or (< (LocalVariables|GetCurrentAngle%20%28Local%29) (LocalVariables|GetBestAngle%20%28Local%29)) (not (Utilities|IsValid (LocalVariables|GetBestTarget%20%28Local%29))))
              (LocalVariables|SetBestTarget%20%28Local%29 (LocalVariables|GetCurrentTarget%20%28Local%29))
              (LocalVariables|SetBestAngle%20%28Local%29 (LocalVariables|GetCurrentAngle%20%28Local%29))))))))
  (return (LocalVariables|GetBestTarget%20%28Local%29)))

(fn SetCurrentTarget
  (params (New%20target :type BP%20Grapple%20Target%20Object%20Reference))
  (if (!= (Variables|Default|GetCurrentTarget) New%20target)
    (Utilities|FlowControl|Sequence
      (:then_0
        (bind _currenttarget (Variables|Default|GetCurrentTarget)
          (:then
            (Default|SetActive _currenttarget false))
          (:else)))
      (:then_1
        (Variables|Default|SetCurrentTarget New%20target))
      (:then_2
        (bind _currenttarget_2 (Variables|Default|GetCurrentTarget)
          (:then
            (Default|SetActive _currenttarget_2 true))
          (:else))))))

(fn AttemptGrapple
  (switch Utilities|FlowControl|Switch|SwitchonEGrappleState (Variables|Default|GetGrappleState)
    (:NewEnumerator0
      (bind _currenttarget (Variables|Default|GetCurrentTarget)
        (:then
          (bind _returnvalue (Game|SpawnActorfromClass "/Game/BluePrints/Grappling/BP_GrappleHook.BP_GrappleHook_C" (Math|Transform|MakeTransform (Utilities|OwnerLocation) "0, 0, 0" "1,1,1") "AlwaysSpawn" 0 _currenttarget 5e+03 0))
          (Variables|Default|SetGrappleHook _returnvalue)
          (bind _returnvalue_2 (Game|SpawnActorfromClass "/Game/BluePrints/Grappling/BP_GrappleLine.BP_GrappleLine_C" (Math|Transform|MakeTransform (Utilities|OwnerLocation) "0, 0, 0" "1,1,1") "AlwaysSpawn" 0 0))
          (bind _output_get (Variables|Default|SetGrappleLine _returnvalue_2))
          (Transformation|AttachComponentToComponent _output_get (Variables|/Script/Engine.Character|GetMesh (Variables|Default|GetOwningCharacter)) "hand_r" "SnapToTarget" "SnapToTarget" "SnapToTarget" true)
          (Class|CableComponent|SetAttachEndto (Variables|/Script/CableComponent.CableActor|GetCableComponent (Variables|Default|GetGrappleLine)) (Variables|Default|GetGrappleHook) "DefaultSceneRoot" "None")
          ;[1 1 1] Not working for now (3/4, 23 min)
          (Transformation|SetActorRotation (Variables|Default|GetOwningCharacter) (Math|Rotator|MakeRotfromZX (Math|Vector|MakeVector 0.0 0.0 1.0) (Utilities|OwnertoTarget)))
          (Variables|Default|SetGrappleState "NewEnumerator1"))
        (:else)))))